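; Gameplay player controller that clears all widgets and sets game-only input when play begins.
; It also holds pause toggle logic that creates or removes a pause menu widget while switching game pause, mouse cursor and input mode, using the widget reference's validity as the state.
; That toggle has no event driving it, so it never runs as the graph stands.
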(event `self.ReceiveBeginPlay`
  ;[1 1 1] Removes Widgets and sets input to game only
  (`WidgetLayoutLibrary.RemoveAllWidgets`)
  (`WidgetBlueprintLibrary.SetInputMode_GameOnly` self))

(fn `UserConstructionScript`)